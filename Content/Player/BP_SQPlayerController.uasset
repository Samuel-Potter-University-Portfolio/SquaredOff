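; BP_SQPlayerController is a player controller that toggles a pause menu and the matching input mode when the Pause action is released.
; It starts in game-only input, and pausing shows the cursor, switches to UI-only input and creates a new PauseMenu widget.
; Unpausing restores game-only input and hides the cursor, but does not remove the widget.
; The Paused flag only tracks state, with no call to pause the game itself.
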(event EventBeginPlay
  (Input|SetInputModeGameOnly self))

(event Input|ActionEvents|InputActionPause
  (params (Key :type Key%20Structure :default "AnyKey"))
  (:Released
    (if (Variables|Default|GetPaused)
      (CallFunction|UnpausePlayer)
      (else
        (CallFunction|PausePlayer)))))

(fn ConstructionScript)

(fn PausePlayer
  (Variables|Default|SetPaused true)
  (Variables|Default|SetbShowMouseCursor true)
  (Input|SetInputModeUIOnly self 0 "DoNotLock")
  (bind _returnvalue (UserInterface|CreateWidget "/Game/UI/PauseMenu.PauseMenu_C" self))
  (UserInterface|Viewport|AddtoViewport _returnvalue 0))

(fn UnpausePlayer
  (Variables|Default|SetPaused false)
  (Variables|Default|SetbShowMouseCursor false)
  (Input|SetInputModeGameOnly self))