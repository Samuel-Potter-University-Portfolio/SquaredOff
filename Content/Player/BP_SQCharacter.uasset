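; BP_SQCharacter is the player character, a cube that visually reflects player colour, health, stun, speed and attacks.
; Construction creates dynamic materials for the core and coloured outline, driven by player state colour and HitFactor.
; Tick eases rotation toward zero when nearly still, toggles stun visibility and high-speed smoke, and randomly spins and shrinks the core during Dash charge.
; Tick also reapplies player colour, destroying the actor if its player state cast fails.
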(event EventTick
  (params (DeltaSeconds :type Float%20%28single-precision%29))
  (|CallParentFunction DeltaSeconds)
  (CallFunction|SmoothRotation)
  (CallFunction|MeshAnimation)
  (|Smokeathighspeed)
  (|EnforcePlayerSettings))

(event EventBeginPlay
  (|CallParentFunction)
  (bind _asbp_sqplayer_state (Utilities|Casting|CastToBP_SQPlayerState (Variables|Default|GetPlayerState)))
  (CallFunction|SetColour (Variables|/Game/Player/BP_SQPlayerState.BP_SQPlayerState_C|GetPlayer%20Colour _asbp_sqplayer_state)))

(fn ConstructionScript
  (Components|Activation|SetActive (Variables|Default|GetJump%20Particle) false false)
  (bind _returnvalue (Rendering|Material|CreateDynamicMaterialInstance (Variables|Default|GetCore) 0 "/Game/Player/Mesh/CubeMat.CubeMat" :!class /Script/Engine.PrimitiveComponent))
  (bind _output_get (Variables|Default|SetCore%20Mat _returnvalue))
  (Rendering|Material|SetMaterial (Variables|Default|GetCore) 0 _output_get)
  (bind _returnvalue_2 (Rendering|Material|CreateDynamicMaterialInstance (Variables|Default|GetColour) 0 "/Game/Player/Mesh/Outline_CMat.Outline_CMat" :!class /Script/Engine.PrimitiveComponent))
  (bind _output_get_2 (Variables|Default|SetColour%20Mat _returnvalue_2))
  (Rendering|Material|SetMaterial (Variables|Default|GetColour) 0 _output_get_2))

(fn ClampRotation
  (params (Rotation :type Rotator))
  (return (Math|Rotator|MakeRotator 0.0 0.0 0.0)))

(fn SmoothRotation
  (bind _rootcomponent (Variables|Transformation|GetRootComponent))
  (bind _returnvalue (Transformation|GetWorldRotation _rootcomponent))
  (if (|NearlyStill)
    (Transformation|SetWorldRotation (Variables|Transformation|GetRootComponent) (Math|Rotator|Lerp(Rotator) _returnvalue (CallFunction|ClampRotation _returnvalue) 0.1 true) false true)))

(fn MeshAnimation
  (|StunAnimation)
  (|Shiftcolourwithhealth)
  (|AttackAnimation (Variables|/Script/SquaredOff.SQAttackComponent|Getcurrent_attack (Variables|Default|Getattack_component))) ; Work around for UE enum issue
)

(fn SetColour
  (params (Colour :type Linear%20Color%20Structure))
  (Rendering|Material|SetVectorParameterValue (Variables|Default|GetColour%20Mat) "Colour" Colour :!class /Script/Engine.MaterialInstanceDynamic))