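; Ranged projectile Blueprint that visualizes its Charge value through four mesh parts and a spinning HitZone.
; The construction script gathers the meshes and gives each a random rotation.
; Each tick splits Charge into quarters, showing completed parts at full scale, growing the current one from a clamped minimum and hiding the rest.
; HitZone yaws continuously, spinning faster as Charge rises.
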(event EventTick
  (params (DeltaSeconds :type Float%20%28single-precision%29))
  (CallFunction|AnimateRotation DeltaSeconds)
  (CallFunction|AnimateParts))

(fn ConstructionScript
  (bind _output_get (Variables|Default|SetMeshes (Utilities|Array|MakeArray (Variables|Default|GetProj%201) (Variables|Default|GetProj%202) (Variables|Default|GetProj%203) (Variables|Default|GetProj%204))))
  (for _array_element _output_get
    (Transformation|SetRelativeRotation _array_element (Math|Random|RandomRotator true) false false)))

(fn AnimateParts
  (bind _charge (Variables|Default|GetCharge))
  (bind (_remainder _returnvalue) (Math|Float|Division(WholeandRemainder) _charge 0.25))
  (for (_array_element _array_index) (Variables|Default|GetMeshes)
    (if (< _array_index _returnvalue)
      (Rendering|SetVisibility _array_element true true)
      (Transformation|SetRelativeScale3D _array_element "1.000000,1.000000,1.000000")
      (elif (== _array_index _returnvalue)
        (Rendering|SetVisibility _array_element true true)
        (Transformation|SetRelativeScale3D _array_element (Math|Conversions|ToVector(Float) (Math|Float|Clamp(Float) (* _remainder 4.0) 0.2)))
        (else
          (Rendering|SetVisibility _array_element false true))))))

(fn AnimateRotation
  (params (Delta%20Seconds :type Float%20%28single-precision%29))
  (Transformation|AddRelativeRotation (Variables|Default|Gethit_zone) (Math|Rotator|MakeRotator 0.0 0.0 (* Delta%20Seconds (+ (* (Variables|Default|GetCharge) 4e+02) 4e+02))) false false))